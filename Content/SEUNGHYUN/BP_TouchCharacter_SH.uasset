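; Player character for a classroom-style scene that presents images and video on a shared screen.
; BeginPlay caches the ScreenView, best-position cameras, slide button and URL widget.
; Keys open HUD inputs, toggle playback and blend the view between pawn and screen camera, with image and focus gated by computer or seat state.
; Req/Res event pairs relay media commands to ScreenView; chair overlap triggers an outline call, while sitting events are stubs.
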(event OnComponentBeginOverlap(CapsuleComponent)
  (params (OverlappedComponent :type Primitive%20Component%20Object%20Reference) (OtherActor :type Actor%20Object%20Reference) (OtherComp :type Primitive%20Component%20Object%20Reference) (OtherBodyIndex :type Integer) (bFromSweep :type Boolean) (SweepResult :type Hit%20Result%20Structure%20%28by%20ref%29))
  (bind _asbp_chair_actor (Utilities|Casting|CastToBP_ChairActor OtherActor))
  (if (Variables|/Game/MobileTest/Blueprint/BP_ChairActor.BP_ChairActor_C|GetIsOtherSitting _asbp_chair_actor)
    (Development|PrintString "IsO")
    (else
      (Variables|Default|SetBP_Chair _asbp_chair_actor)
      (Default|IsntOwnSitonOutline (Variables|Default|GetBP_Chair))
      (Development|PrintString "앉는다"))))

(event OnComponentEndOverlap(CapsuleComponent)
  (params (OverlappedComponent :type Primitive%20Component%20Object%20Reference) (OtherActor :type Actor%20Object%20Reference) (OtherComp :type Primitive%20Component%20Object%20Reference) (OtherBodyIndex :type Integer))
  (Utilities|Casting|CastToBP_ChairActor OtherActor))

(event Custom|ReqSwitchVideo
  ;[1 1 1] [ Video ] P키 한번 누르면 멈추고 다시 누르면 다시 재생
  (CallFunction|ResSwitchVideoState))

(event Custom|ResSwitchVideoState
  ;[1 1 1] [ Video ] P키 한번 누르면 멈추고 다시 누르면 다시 재생
  (Default|SwitchVideo (Variables|Default|GetScreenView)))

(event Custom|FrontComputerWidget
  (bind _asbp_touch_hud (Utilities|Casting|CastToBP_TouchHud (HUD|GetHUD (Game|GetPlayerController 0))))
  (Default|ShowComputerWidget _asbp_touch_hud))

(event Custom|SetCameraPositionCam
  (switch Utilities|FlowControl|Switch|SwitchonEN_CameraFocus (Variables|Default|GetFocusOn)
    (:NewEnumerator1
      (Game|Player|SetViewTargetwithBlend (Game|GetPlayerController 0) (Game|Player|GetPlayerPawn 0) 1.0 "VTBlend_Linear" 0.0 false)
      (Variables|Default|SetFocusOn "NewEnumerator2"))
    (:NewEnumerator2
      (Game|Player|SetViewTargetwithBlend (Game|GetPlayerController 0) (Variables|Default|GetBestPositionCameraCom) 1.0 "VTBlend_Linear" 0.0 false)
      (Variables|Default|SetFocusOn "NewEnumerator1"))))

(event Custom|OnSitting
  (for _array_element (Collision|GetOverlappingActors (Variables|Default|GetCapsuleComponent) "/Game/MobileTest/Blueprint/BP_ChairActor.BP_ChairActor_C" :!class /Script/Engine.PrimitiveComponent)
    (bind _asbp_chair_actor (Utilities|Casting|CastToBP_ChairActor _array_element))
    (if (Variables|/Game/MobileTest/Blueprint/BP_ChairActor.BP_ChairActor_C|GetIsOtherSitting _asbp_chair_actor)
      _)))

(event Custom|OffSitting)

(event EventBeginPlay
  (|CallParentFunction)
  (Utilities|FlowControl|Sequence
    (:then_0
      (bind _returnvalue (Actor|GetActorOfClass "/Game/SEUNGHYUN/Image/BP_ScreenView.BP_ScreenView_C"))
      (Variables|Default|SetScreenView _returnvalue)
      (bind _returnvalue_2 (Actor|GetActorOfClass "/Game/SEUNGHYUN/Video/BP_BestPositionCamera.BP_BestPositionCamera_C"))
      (Variables|Default|SetBestPositionCamera _returnvalue_2)
      (bind _returnvalue_3 (Actor|GetActorOfClass "/Game/SEUNGHYUN/Image/BTN_ImageSlideButton.BTN_ImageSlideButton_C"))
      (Variables|Default|SetImageSlideButton _returnvalue_3)
      (bind _returnvalue_4 (Actor|GetActorOfClass "/Game/SEUNGHYUN/Video/BP_BestPositionCamera_Computer.BP_BestPositionCamera_Computer_C"))
      (Variables|Default|SetBestPositionCameraCom _returnvalue_4)
      (bind _assh_hud (Utilities|Casting|CastToSH_HUD (HUD|GetHUD (Game|GetPlayerController 0))))
      (Variables|Default|SetInput%20Video%20Url%20Widget (Variables|/Game/SEUNGHYUN/Image/SH_HUD.SH_HUD_C|GetInputVideoUrlWidget _assh_hud)))))

(event Input|KeyboardEvents|I
  (params (Key :type Key%20Structure))
  ;[1 1 1] [ Image ] I 키 누르면 허드에 이미지 위젯 보여줌
  (:Pressed
    ;;[1 1 1] UserInfo가 교수이면
    (if (Variables|Default|GetIsFrontComputer)
      (Default|VisibleButton (Variables|Default|GetImageSlideButton))
      (bind _assh_hud (Utilities|Casting|CastToSH_HUD (HUD|GetHUD (Game|GetPlayerController 0))))
      (Default|ImageRender _assh_hud))))

(event Input|KeyboardEvents|P
  (params (Key :type Key%20Structure))
  ;[1 1 1] [ Video ] P키 한번 누르면 멈추고 다시 누르면 다시 재생
  (:Pressed
    (if (Variables|Default|GetCanPlay)
      (CallFunction|ReqSwitchVideo))))

(event Input|KeyboardEvents|V
  (params (Key :type Key%20Structure))
  ;[1 1 1] [ Video ] V키 누르면 비디오 url 위젯 보여줌
  (:Pressed
    (bind _assh_hud (Utilities|Casting|CastToSH_HUD (HUD|GetHUD (Game|GetPlayerController 0))))
    (Default|ShowVideoUrlWidget _assh_hud)))

(event Input|KeyboardEvents|F
  (params (Key :type Key%20Structure))
  ;[1 1 1] F누르면 CameraFocus 전환
  (:Pressed
    (if (or (Variables|Default|GetIsFrontComputer) (Variables|Default|GetIsSitting))
      (switch Utilities|FlowControl|Switch|SwitchonEN_CameraFocus (Variables|Default|GetFocusOn)
        (:NewEnumerator0
          (Game|Player|SetViewTargetwithBlend (Game|GetPlayerController 0) (Variables|Default|GetBestPositionCamera) 1.0 "VTBlend_Linear" 0.0 false)
          (Variables|Default|SetFocusOn "NewEnumerator1"))
        (:NewEnumerator1
          (Game|Player|SetViewTargetwithBlend (Game|GetPlayerController 0) (Game|Player|GetPlayerPawn 0) 1.0 "VTBlend_Linear" 0.0 false)
          (Variables|Default|SetFocusOn "NewEnumerator0"))))))

(event Custom|OnThrobber
  ;[1 1 1] Throbber
  (CallFunction|OnThrobber2))

(event Custom|ReqImage
  (params (ImageURL :type String) (URL_Length :type Integer))
  ;[1 1 1] Image
  (CallFunction|ResImage ImageURL URL_Length))

(event Custom|ReqVideo
  (params (VideoURL :type String))
  ;[1 1 1] Video
  (CallFunction|ResVideo VideoURL))

(event Custom|ResVideo
  (params (VideoURL :type String))
  ;[1 1 1] Video
  (Default|SetVideo (Variables|Default|GetScreenView) VideoURL))

(event Custom|ReqBefore
  (CallFunction|ResBefore))

(event Custom|ResImage
  (params (ImageURL :type String) (URL_Length :type Integer))
  ;[1 1 1] Image
  (Default|SetImage (Variables|Default|GetScreenView) ImageURL URL_Length))

(event Custom|OnThrobber_2
  ;[1 1 1] Throbber
  (Default|VisibleLoadingWidget (Variables|Default|GetScreenView)))

(event Custom|ResBefore
  (Default|PressBeforeButton2 (Variables|Default|GetScreenView)))

(event Custom|ReqLater
  (CallFunction|ResLater))

(event Custom|ResLater
  (Default|PressAfterButton2 (Variables|Default|GetScreenView)))

(fn ConstructionScript
  (|CallParentFunction))