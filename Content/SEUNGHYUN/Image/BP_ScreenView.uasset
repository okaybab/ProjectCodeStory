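; In-world screen actor that shows downloaded images as a slideshow or streams a video on its Cube mesh.
; SetImage downloads each URL into a texture map, and SetMT applies textures through a dynamic material instance.
; Slide-button presses forward requests to BP_TouchCharacter_SH, while separate events step the clamped image index.
; SetVideo opens a stream and reports success to the character; play/pause briefly flashes button icons via timers.
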(event Custom|SetImage
  (params (ImageURL :type String))
  (bind _texturemap (Variables|Default|GetTextureMap))
  (bind _returnvalue (Utilities|Array|Add (Variables|Default|GetImageURL) ImageURL))
  (bind _texture (|DownloadImage (Utilities|Array|Get(acopy) (Variables|Default|GetImageURL) _returnvalue))
    (:OnSuccess
      (Utilities|Map|Add _texturemap (Utilities|Array|Get(acopy) (Variables|Default|GetImageURL) (Variables|Default|GetDownloadCount)) _texture)
      (Math|Integer|IncrementInt (Variables|Default|GetDownloadCount)
        (:%20%20
          (CallFunction|HiddenLoadingWidget)
          (CallFunction|SetMT (.Value (Utilities|Map|Find _texturemap (Utilities|Array|Get(acopy) (Variables|Default|GetImageURL))))))))))

(event Custom|SetVideo
  (params (VideoURL :type String))
  (bind _videosource (Variables|Default|GetVideoSource))
  (Variables|/Script/MediaAssets.StreamMediaSource|SetStreamUrl _videosource VideoURL)
  (Utilities|IsValid _videosource
    (:Is%20Valid
      (CallFunction|SetVideoMT)
      (bind _returnvalue (Media|MediaPlayer|OpenSource (Variables|Default|GetVideoPlayer) "/Game/SEUNGHYUN/Video/VIdeoSource.VIdeoSource"))
      (bind _asbp_touch_character_sh (Utilities|Casting|CastToBP_TouchCharacter_SH (Game|Player|GetPlayerPawn 0)))
      (Variables|/Game/SEUNGHYUN/BP_TouchCharacter_SH.BP_TouchCharacter_SH_C|SetCanPlay _asbp_touch_character_sh _returnvalue))
    (:Is%20Not%20Valid
      (Development|PrintString "URL not valid" true true "(R=1.000000,G=0.020335,B=0.050181,A=1.000000)" 5e+01))))

(event Custom|PressBeforeButton
  (bind _asbp_touch_character_sh (Utilities|Casting|CastToBP_TouchCharacter_SH (Game|GetPlayerCharacter 0)))
  (Default|ReqBefore _asbp_touch_character_sh))

(event Custom|PressAfterButton
  (bind _asbp_touch_character_sh (Utilities|Casting|CastToBP_TouchCharacter_SH (Game|GetPlayerCharacter 0)))
  (Default|ReqLater _asbp_touch_character_sh))

(event Custom|PressAfterButton2
  (bind _output_get (Variables|Default|SetImageIndex (Math|Integer|Clamp(Integer) (+ (Variables|Default|GetImageIndex) 1) 0 (- (Utilities|Array|Length (Variables|Default|GetImageURL)) 1))))
  (Development|PrintString (Utilities|Array|Get(acopy) (Variables|Default|GetImageURL) _output_get) true true "(R=0.000000,G=0.660000,B=1.000000,A=1.000000)" 333.0)
  (CallFunction|SetMT (.Value (Utilities|Map|Find (Variables|Default|GetTextureMap) (Utilities|Array|Get(acopy) (Variables|Default|GetImageURL) _output_get)))))

(event Custom|PressBeforeButton2
  (bind _output_get (Variables|Default|SetImageIndex (Math|Integer|Clamp(Integer) (- (Variables|Default|GetImageIndex) 1) 0 (- (Utilities|Array|Length (Variables|Default|GetImageURL)) 1))))
  (Development|PrintString (Utilities|Array|Get(acopy) (Variables|Default|GetImageURL) _output_get) true true "(R=0.000000,G=0.660000,B=1.000000,A=1.000000)" 333.0)
  (CallFunction|SetMT (.Value (Utilities|Map|Find (Variables|Default|GetTextureMap) (Utilities|Array|Get(acopy) (Variables|Default|GetImageURL) _output_get)))))

(event EventBeginPlay
  (Utilities|FlowControl|Sequence
    (:then_0
      (bind _returnvalue (Actor|GetActorOfClass "/Game/SEUNGHYUN/Image/BTN_ImageSlideButton.BTN_ImageSlideButton_C"))
      (EventDispatchers|BindEventtoEventDispatcherBefore _returnvalue (EventDispatchers|CreateEvent :!event Custom|PressBeforeButton))
      (EventDispatchers|BindEventtoEventDispatcherLater _returnvalue (EventDispatchers|CreateEvent :!event Custom|PressAfterButton)))
    (:then_1
      (bind _returnvalue_2 (Actor|GetActorOfClass "/Game/SEUNGHYUN/Image/UploadImage.UploadImage_C"))
      (Variables|Default|SetUploadImage _returnvalue_2)
      (bind _returnvalue_3 (Actor|GetActorOfClass "/Game/SEUNGHYUN/Image/UploadImage.UploadImage_C"))
      (Variables|Default|SetUploadImage _returnvalue_3))))

(fn ConstructionScript)

(fn SetVideoMT
  (Rendering|Material|SetMaterial (Variables|Default|GetCube) 0 "/Game/SEUNGHYUN/Video/MT_Video.MT_Video"))

(fn SetImageMT
  (Rendering|Material|SetMaterial (Variables|Default|GetCube) 0 "/Game/SEUNGHYUN/Image/MT_ImageView.MT_ImageView"))

(fn VisibleLoadingWidget
  (Rendering|SetVisibility (Variables|Default|GetLoadingWidget) true false))

(fn HiddenLoadingWidget
  (Rendering|SetVisibility (Variables|Default|GetLoadingWidget) false false))

(fn SetMT
  (params (InputObject :type Texture%20Object%20Reference))
  (bind _returnvalue (Rendering|Material|CreateDynamicMaterialInstance (Variables|Default|GetCube) 0 "/Game/SEUNGHYUN/Image/MT_ImageView.MT_ImageView" "None" :!class /Script/Engine.PrimitiveComponent))
  (Utilities|IsValid InputObject
    (:Is%20Valid
      (Rendering|Material|SetTextureParameterValue _returnvalue "Texture" InputObject))
    (:Is%20Not%20Valid
      (Development|PrintString "Material Not Valid" true true "(R=0.000000,G=0.660000,B=1.000000,A=1.000000)" 5e+01))))

(fn PauseVideo
  (Sequencer|Player|Pause (Variables|Default|GetVideoPlayer))
  (Utilities|Time|SetTimerbyFunctionName 0 "SetStopButtonVisible" 0.01)
  (Utilities|Time|SetTimerbyFunctionName 0 "SetStopButtonHidden" 0.3)
  (Variables|Default|SetIsPlay false))

(fn PlayVideo
  (Media|MediaPlayer|Play (Variables|Default|GetVideoPlayer) :!class /Script/MediaAssets.MediaPlayer)
  (Utilities|Time|SetTimerbyFunctionName 0 "SetPlayButtonVisible" 0.01)
  (Utilities|Time|SetTimerbyFunctionName 0 "SetPlayButtonHidden" 0.3)
  (Variables|Default|SetIsPlay true))

(fn SwitchVideo
  (if (Variables|Default|GetIsPlay)
    (CallFunction|PauseVideo)
    (else
      (CallFunction|PlayVideo))))

(fn SetPlayButtonVisible
  (Rendering|SetVisibility (Variables|Default|GetPlayButton) true false))

(fn SetStopButtonVisible
  (Rendering|SetVisibility (Variables|Default|GetStopButton) true false))

(fn SetPlayButtonHidden
  (Rendering|SetVisibility (Variables|Default|GetPlayButton) false false))

(fn SetStopButtonHidden
  (Rendering|SetVisibility (Variables|Default|GetStopButton) false false))

(fn OnRepGetURLLength)