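; Mesh capture actor in a mobile test folder that displays a character built from a skeletal Body mesh and a static Hair mesh.
; Simple functions set each mesh and return the current pair.
; A separate SetBody event swaps the Body mesh with a pose reinit, only on the Remote (non-authority) side.
; The file contains no capture logic, and its BeginPlay and overlap events are empty.
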(event Custom|SetBody
  (params (NewParam :type Skeletal%20Mesh%20Object%20Reference))
  (Networking|SwitchHasAuthority
    (:Remote
      (Class|SkinnedMeshComponent|SetSkeletalMesh (Variables|Default|Getbody) NewParam true))))

(event EventBeginPlay)

(event Collision|EventActorBeginOverlap
  (params (OtherActor :type Actor%20Object%20Reference)))

(fn ConstructionScript)

(fn SetBodyMesh
  (params (skeletalMesh :type Skeletal%20Mesh%20Object%20Reference))
  (Class|SkinnedMeshComponent|SetSkeletalMesh (Variables|Default|Getbody) skeletalMesh true))

(fn SetHairMesh
  (params (StaticMesh :type Static%20Mesh%20Object%20Reference))
  (Components|StaticMesh|SetStaticMesh (Variables|Default|Gethair) StaticMesh))

(fn GetBodyHairMesh
  (return (Variables|/Script/Engine.SkinnedMeshComponent|GetSkeletalMesh (Variables|Default|Getbody)) (Variables|/Script/Engine.StaticMeshComponent|GetStaticMesh (Variables|Default|Gethair))))