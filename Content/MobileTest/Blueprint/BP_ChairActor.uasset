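; BP_ChairActor is a chair that can show an outline highlight and a widget, which starts hidden.
; IsntOwnSit_OnOutline and IsntOwnSit_OffOutline toggle both together.
; The outline is a runtime duplicate of the static mesh with a dynamic M_Outline_Inst material taking Color and Scale, guarded by HasOutline.
; Capsule overlap and cursor events are empty, and their former player and occupancy checks are disconnected.
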(event OnBeginCursorOver(Capsule)
  (params (TouchedComponent :type Primitive%20Component%20Object%20Reference))
  ;[1 1 1] Mouse Cursor
)

(event OnEndCursorOver(Capsule)
  (params (TouchedComponent :type Primitive%20Component%20Object%20Reference))
  ;[1 1 1] Mouse Cursor
)

(event OnComponentBeginOverlap(Capsule)
  (params (OverlappedComponent :type Primitive%20Component%20Object%20Reference) (OtherActor :type Actor%20Object%20Reference) (OtherComp :type Primitive%20Component%20Object%20Reference) (OtherBodyIndex :type Integer) (bFromSweep :type Boolean) (SweepResult :type Hit%20Result%20Structure%20%28by%20ref%29)))

(event OnComponentEndOverlap(Capsule)
  (params (OverlappedComponent :type Primitive%20Component%20Object%20Reference) (OtherActor :type Actor%20Object%20Reference) (OtherComp :type Primitive%20Component%20Object%20Reference) (OtherBodyIndex :type Integer)))

(event Custom|CreateOutline
  (if (not (Variables|Default|GetHasOutline))
    (bind _returnvalue (AddComponent|AddStaticMeshComponent true (Transformation|GetWorldTransform (Variables|Default|GetStaticMesh))))
    (bind _output_get (Variables|Default|SetMeshComponent _returnvalue))
    (Components|StaticMesh|SetStaticMesh _output_get (Variables|/Script/Engine.StaticMeshComponent|GetStaticMesh (Variables|Default|GetStaticMesh)))
    (bind _returnvalue_2 (Rendering|Material|CreateDynamicMaterialInstance (Variables|Default|GetMeshComponent) 0 "/Game/Assets/Outline/M_Outline_Inst.M_Outline_Inst" "None" :!class /Script/Engine.PrimitiveComponent))
    (Rendering|Material|SetVectorParameterValue _returnvalue_2 "Color" (Variables|Default|GetColor) :!class /Script/Engine.MaterialInstanceDynamic)
    (Rendering|Material|SetScalarParameterValue _returnvalue_2 "Scale" (Variables|Default|GetScale) :!class /Script/Engine.MaterialInstanceDynamic)
    (Variables|Default|SetHasOutline true)))

(event Custom|DeleteOutline
  (bind _meshcomponent (Variables|Default|GetMeshComponent))
  (Utilities|IsValid _meshcomponent
    (:Is%20Valid
      (Components|DestroyComponent _meshcomponent)
      (Variables|Default|SetHasOutline false))))

(event Custom|IsntOwnSit_OffOutline
  (CallFunction|DeleteOutline)
  (Rendering|SetVisibility (Variables|Default|GetWidget) false false))

(event Custom|IsntOwnSit_OnOutline
  (CallFunction|CreateOutline)
  (Rendering|SetVisibility (Variables|Default|GetWidget) true false))

(event EventBeginPlay
  (Rendering|SetVisibility (Variables|Default|GetWidget) false false))

(fn ConstructionScript)