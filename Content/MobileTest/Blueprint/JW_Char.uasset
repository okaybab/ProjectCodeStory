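; Mobile test player character for a cosmetic item shop, with owned items and a money balance.
; BeginPlay grants 100 money to player 0, binds HUD Buy/Wear events and seeds default body and hair from DataTables.
; Buying checks ownership and GameInstance money locally; the HTTP purchase call is disconnected.
; Wearing sends a server RPC to swap the skeletal mesh, but looks up an empty item key, and hair swapping is unwired.
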(event Custom|OnBuyItem
  (bind _asbp_touch_hud (Utilities|Casting|CastToBP_TouchHud (HUD|GetHUD (Game|GetPlayerController 0))))
  (bind _itemiconstruct (Default|GetItemStruct _asbp_touch_hud))
  (CallFunction|AddStoreItem _itemiconstruct))

(event Custom|ReqWearItem
  (params (NewParam :type Object%20Object%20Reference))
  ;[1 0 0] Server
  (CallFunction|ResWearItem NewParam))

(event Custom|ResWearItem
  (params (NewParam :type Object%20Object%20Reference))
  (bind _asskeletal_mesh (Utilities|Casting|CastToSkeletalMesh NewParam))
  (Class|SkinnedMeshComponent|SetSkeletalMesh (Variables|Character|GetMesh) _asskeletal_mesh true)
  (Development|PrintString "setbody" true true "(R=0.000000,G=0.660000,B=1.000000,A=1.000000)" 6e+01))

(event Custom|OnWearItem
  (bind _ownitem (Variables|Default|GetOwnItem))
  (bind (_value _returnvalue) (Utilities|Map|Find _ownitem ""))
  (bind _asbp_touch_hud (Utilities|Casting|CastToBP_TouchHud (HUD|GetHUD (Game|GetPlayerController 0))))
  (Default|GetItemName _asbp_touch_hud)
  (Utilities|FlowControl|Sequence
    (:then_0
      (if _returnvalue
        (CallFunction|ReqWearItem (.itemobject _value))))
    (:then_1
      (if (.ReturnValue (Utilities|Map|Find _ownitem ""))
        _))))

(event Custom|커스텀이벤트_0)

(event EventBeginPlay
  (Utilities|FlowControl|Sequence
    (:then_0
      (bind _outactors (Actor|GetAllActorsOfClass "/Game/MyHttpActor.MyHttpActor_C"))
      (for _array_element _outactors
        (Variables|Default|SetHttpActor _array_element))
      (if (== (Game|GetPlayerCharacter 0) self) :!label _label
        (bind _asmee_game_instance (Utilities|Casting|CastToMee_GameInstance (Game|GetGameInstance)))
        (Class|MeeGameInstance|SetMoney _asmee_game_instance 100)
        (Development|PrintString (Utilities|GetDisplayName _asmee_game_instance) false false "(R=1.000000,G=0.004704,B=0.000000,A=1.000000)" 62.0)))
    (:then_1
      (goto _label))
    (:then_2
      (EventDispatchers|BindEventtoEventDispatcherBuyButton (EventDispatchers|CreateEvent :!event Custom|OnBuyItem))
      (EventDispatchers|BindEventtoEventDispatcherWearButton (EventDispatchers|CreateEvent :!event Custom|OnWearItem))
      (bind _returnvalue (Utilities|GetDataTableRow "/Game/MobileTest/Data/DT_BodyChar.DT_BodyChar" "item0")
        (:then
          (Utilities|Map|Add (Variables|Default|GetOwnItem) "item0" (Utilities|Struct|MakeST_ShopOwnStruct (.price _returnvalue) (.mesh _returnvalue) true "Body" "item0"))
          (bind _returnvalue_2 (Utilities|GetDataTableRow "/Game/MobileTest/Data/DT_ShopHair.DT_ShopHair" "item10")
            (:then
              (Utilities|Map|Add (Variables|Default|GetOwnItem) "item10" (Utilities|Struct|MakeST_ShopOwnStruct (.price _returnvalue_2) (.mesh _returnvalue_2) true "Hair" "item10")))))))))

(fn ConstructionScript)

(fn AddStoreItem
  (params (AddItem :type ST%20Shop%20Own%20Struct%20Structure))
  (bind (_itemprice _itemobject _itemname) (Utilities|Struct|BreakST_ShopOwnStruct AddItem))
  (bind (_itemprice_2 _itemobject_2 _itemtype _itemname_2) (Utilities|Struct|BreakST_ShopOwnStruct AddItem))
  (bind _asmee_game_instance (Utilities|Casting|CastToMee_GameInstance (Game|GetGameInstance)))
  (LocalVariables|SetLocalGameInstance _asmee_game_instance)
  (Utilities|IsValid _itemobject
    (:Is%20Valid
      ;[1 1 1] server에서 소유한값 찾기
      (bind _isown (CallFunction|IsOwn _itemname))
      (if _isown
        (Development|PrintString "가지고 있음")
        (else
          (bind _returnvalue (Class|MeeGameInstance|GetMoney (LocalVariables|GetLocalGameInstance)))
          (if (>= (- _returnvalue _itemprice) 0)
            (Class|MeeGameInstance|SetMoney (LocalVariables|GetLocalGameInstance) (- _returnvalue _itemprice))
            (Utilities|Map|Add (Variables|Default|GetOwnItem) _itemname_2 (Utilities|Struct|MakeST_ShopOwnStruct _itemprice_2 _itemobject_2 true _itemtype _itemname_2))
            (Development|PrintString "AddItem")
            (else
              (Development|PrintString "돈이 없음"))))))))

(fn IsOwn
  (params (ItemName :type String))
  (bind _ownitem (Variables|Default|GetOwnItem))
  (bind _returnvalue (Utilities|Map|Find _ownitem ItemName))
  (if _returnvalue
    (return _returnvalue)
    (else
      (return _returnvalue))))