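; Player character for a mobile test with a body and hair cosmetic shop.
; On BeginPlay it loads game-instance user data, equips saved items from data tables and fills an owned-item map, typing inventory items by code substring.
; HUD buy events check ownership and money locally, with the HTTP purchase call left disconnected.
; Wearing goes through a Server event to a Client event that sets RepNotify mesh variables, whose OnReps apply the meshes.
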(event Custom|OnBuyItem
  (bind _asbp_touch_hud (Utilities|Casting|CastToBP_TouchHud (HUD|GetHUD (Game|GetPlayerController 0))))
  (bind _itemiconstruct (Default|GetItemStruct _asbp_touch_hud))
  (CallFunction|AddStoreItem _itemiconstruct))

(event Custom|ReqWearItem
  (params (ItemMesh :type Object%20Object%20Reference%20%28by%20ref%29) (ItemEnum :type Enum_ShopItem%20Enum :default "NewEnumerator0"))
  ;[1 0 0] Server
  (CallFunction|ResWearItem ItemMesh ItemEnum))

(event Custom|ResWearItem
  (params (ItemMesh :type Object%20Object%20Reference%20%28by%20ref%29) (ItemEnum :type Enum_ShopItem%20Enum :default "NewEnumerator0"))
  ;[1 1 1] Client
  (switch Utilities|FlowControl|Switch|SwitchonEnum_ShopItem ItemEnum
    (:NewEnumerator0
      (bind _asskeletal_mesh (Utilities|Casting|CastToSkeletalMesh ItemMesh))
      (Variables|Default|Setbodymesh _asskeletal_mesh))
    (:NewEnumerator1
      (bind _asstatic_mesh (Utilities|Casting|CastToStaticMesh ItemMesh))
      (Variables|Default|Sethairmesh _asstatic_mesh))))

(event Custom|OnWearItem
  (bind _asbp_touch_hud (Utilities|Casting|CastToBP_TouchHud (HUD|GetHUD (Game|GetPlayerController 0))))
  (bind _stringmesh (Default|GetItemName _asbp_touch_hud))
  (bind _keys (Utilities|Map|Keys _stringmesh))
  (for _array_element _keys
    (if (.ReturnValue (Utilities|Map|Find (Variables|Default|GetOwnItem) (.Value (Utilities|Map|Find _stringmesh _array_element))))
      (CallFunction|ReqWearItem (.itemobject (.Value (Utilities|Map|Find (Variables|Default|GetOwnItem) (.Value (Utilities|Map|Find _stringmesh _array_element))))) (.itemtype (.Value (Utilities|Map|Find (Variables|Default|GetOwnItem) (.Value (Utilities|Map|Find _stringmesh _array_element)))))))))

(event EventBeginPlay
  (Utilities|FlowControl|Sequence
    (:then_0
      (bind _outactors (Actor|GetAllActorsOfClass "/Game/MyHttpActor.MyHttpActor_C"))
      (for _array_element _outactors
        (Variables|Default|SetHttpActor _array_element))
      (if (== (Game|GetPlayerCharacter 0) self) :!label _label
        (bind _asmee_game_instance (Utilities|Casting|CastToMee_GameInstance (Game|GetGameInstance)))
        (bind (_outequipmentbody _outequipmenthair _outmoney _outinventory) (Class|MeeGameInstance|GetUserData _asmee_game_instance))
        (Utilities|FlowControl|Sequence
          (:then_0
            (bind _returnvalue (Utilities|GetDataTableRow "/Game/MobileTest/Data/DT_BodyChar.DT_BodyChar" (Utilities|String|StringToName _outequipmenthair))
              (:then
                (CallFunction|ReqWearItem (.mesh _returnvalue) "NewEnumerator0"))))
          (:then_1
            (bind _returnvalue_2 (Utilities|GetDataTableRow "/Game/MobileTest/Data/DT_ShopHair.DT_ShopHair" (Utilities|String|StringToName _outequipmentbody))
              (:then
                (CallFunction|ReqWearItem (.mesh _returnvalue_2) "NewEnumerator1"))))
          (:then_2
            (for _array_element_2 _outinventory
              (switch Utilities|FlowControl|Switch|SwitchonEnum_ShopItem (Utilities|Select :Index (Math|Integer|Clamp(Integer) (/ (Math|Conversions|ToInteger(Byte) (Utilities|String|GetSubstring _array_element_2 4 2)) 10) 0 1) :Option%200 "NewEnumerator0" :Option%201 "NewEnumerator1")
                (:NewEnumerator0
                  (bind _returnvalue_3 (Utilities|GetDataTableRow "/Game/MobileTest/Data/DT_BodyChar.DT_BodyChar" (Utilities|String|StringToName _array_element_2))
                    (:then
                      (CallFunction|AddOwnItem (Utilities|Struct|MakeST_ShopOwnStruct (.price _returnvalue_3) (.mesh _returnvalue_3) true (Utilities|Select :Index (Math|Integer|Clamp(Integer) (/ (Math|Conversions|ToInteger(Byte) (Utilities|String|GetSubstring _array_element_2 4 2)) 10) 0 1) :Option%200 "NewEnumerator0" :Option%201 "NewEnumerator1") _array_element_2)))))
                (:NewEnumerator1
                  (bind _returnvalue_4 (Utilities|GetDataTableRow "/Game/MobileTest/Data/DT_ShopHair.DT_ShopHair" (Utilities|String|StringToName _array_element_2))
                    (:then
                      (CallFunction|AddOwnItem (Utilities|Struct|MakeST_ShopOwnStruct (.price _returnvalue_4) (.mesh _returnvalue_4) true (Utilities|Select :Index (Math|Integer|Clamp(Integer) (/ (Math|Conversions|ToInteger(Byte) (Utilities|String|GetSubstring _array_element_2 4 2)) 10) 0 1) :Option%200 "NewEnumerator0" :Option%201 "NewEnumerator1") _array_element_2)))))))))))
    (:then_1
      (goto _label))
    (:then_2
      (EventDispatchers|BindEventtoEventDispatcherBuyButton (EventDispatchers|CreateEvent :!event Custom|OnBuyItem))
      (EventDispatchers|BindEventtoEventDispatcherWearButton (EventDispatchers|CreateEvent :!event Custom|OnWearItem)))))

(fn ConstructionScript)

(fn AddStoreItem
  (params (AddItem :type ST%20Shop%20Own%20Struct%20Structure))
  (bind (_itemprice _itemobject _itemtype _itemname) (Utilities|Struct|BreakST_ShopOwnStruct AddItem))
  (bind (_itemprice_2 _itemobject_2 _itemtype_2 _itemname_2) (Utilities|Struct|BreakST_ShopOwnStruct AddItem))
  (bind _asmee_game_instance (Utilities|Casting|CastToMee_GameInstance (Game|GetGameInstance)))
  (LocalVariables|SetLocalGameInstance _asmee_game_instance)
  (Utilities|IsValid _itemobject
    (:Is%20Valid
      ;[1 1 1] server에서 소유한값 찾기
      (bind _isown (CallFunction|IsOwn _itemname))
      (if _isown
        (Development|PrintString "가지고 있음")
        (else
          (bind _returnvalue (Class|MeeGameInstance|GetMoney (LocalVariables|GetLocalGameInstance)))
          (if (>= (- _returnvalue _itemprice) 0)
            (Class|MeeGameInstance|SetMoney (LocalVariables|GetLocalGameInstance) (- _returnvalue _itemprice))
            (Utilities|Map|Add (Variables|Default|GetOwnItem) _itemname_2 (Utilities|Struct|MakeST_ShopOwnStruct _itemprice_2 _itemobject_2 true _itemtype_2 _itemname_2))
            (Development|PrintString "AddItem")
            (else
              (Development|PrintString "돈이 없음"))))))))

(fn IsOwn
  (params (ItemName :type String))
  (bind _ownitem (Variables|Default|GetOwnItem))
  (bind _returnvalue (Utilities|Map|Find _ownitem ItemName))
  (if _returnvalue
    (return _returnvalue)
    (else
      (return _returnvalue))))

(fn OnRepBodymesh
  (Class|SkinnedMeshComponent|SetSkeletalMesh (Variables|Character|GetMesh) (Variables|Default|Getbodymesh) true))

(fn OnRepHairmesh
  (Components|StaticMesh|SetStaticMesh (Variables|Default|Gethair) (Variables|Default|Gethairmesh)))

(fn GetMesh
  (return (Variables|/Script/Engine.SkinnedMeshComponent|GetSkeletalMesh (Variables|Character|GetMesh)) (Variables|/Script/Engine.StaticMeshComponent|GetStaticMesh (Variables|Default|Gethair))))

(fn AddOwnItem
  (params (Value :type ST%20Shop%20Own%20Struct%20Structure%20%28by%20ref%29))
  (Utilities|Map|Add (Variables|Default|GetOwnItem) (Utilities|Struct|BreakST_ShopOwnStruct Value) Value))