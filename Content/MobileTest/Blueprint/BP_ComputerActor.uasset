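; BP_ComputerActor is a computer prop that tells the local player's BP_TouchCharacter_SH whether it is in front of the computer.
; When that character exits the Box, the sign of the Arrow's forward Y times the character's Y offset from the Arrow gives the side.
; The result sets IsFrontComputer and FocusOn, then calls FrontComputerWidget on the character.
; The check uses only the world Y axis, and begin overlap does nothing.
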(event OnComponentBeginOverlap(Box)
  (params (OverlappedComponent :type Primitive%20Component%20Object%20Reference) (OtherActor :type Actor%20Object%20Reference) (OtherComp :type Primitive%20Component%20Object%20Reference) (OtherBodyIndex :type Integer) (bFromSweep :type Boolean) (SweepResult :type Hit%20Result%20Structure%20%28by%20ref%29)))

(event OnComponentEndOverlap(Box)
  (params (OverlappedComponent :type Primitive%20Component%20Object%20Reference) (OtherActor :type Actor%20Object%20Reference) (OtherComp :type Primitive%20Component%20Object%20Reference) (OtherBodyIndex :type Integer))
  (bind _arrow (Variables|Default|GetArrow))
  (bind _asbp_touch_character_sh (Utilities|Casting|CastToBP_TouchCharacter_SH OtherActor))
  (if (== _asbp_touch_character_sh (Game|GetPlayerCharacter 0))
    (if (> (* (.y (Math|Vector|GetForwardVector _arrow)) (- (.y (Transformation|GetActorLocation _asbp_touch_character_sh)) (.y (Transformation|GetWorldLocation _arrow)))) 0.0)
      (Variables|/Game/SEUNGHYUN/BP_TouchCharacter_SH.BP_TouchCharacter_SH_C|SetIsFrontComputer _asbp_touch_character_sh true)
      (Variables|/Game/SEUNGHYUN/BP_TouchCharacter_SH.BP_TouchCharacter_SH_C|SetFocusOn _asbp_touch_character_sh "NewEnumerator2")
      (Default|FrontComputerWidget _asbp_touch_character_sh)
      (else
        (Variables|/Game/SEUNGHYUN/BP_TouchCharacter_SH.BP_TouchCharacter_SH_C|SetIsFrontComputer _asbp_touch_character_sh false)
        (Variables|/Game/SEUNGHYUN/BP_TouchCharacter_SH.BP_TouchCharacter_SH_C|SetFocusOn _asbp_touch_character_sh "NewEnumerator1")
        (Default|FrontComputerWidget _asbp_touch_character_sh)))))

(event EventBeginPlay)

(event Collision|EventActorBeginOverlap
  (params (OtherActor :type Actor%20Object%20Reference)))

(event EventTick
  (params (DeltaSeconds :type Float%20%28single-precision%29)))

(fn ConstructionScript)