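; BP_TouchHud is an actor that owns the W_TouchHud widget in the mobile test and holds the currently selected item's data.
; It creates the widget and adds it to the viewport on BeginPlay.
; SetItemStruct stores the item struct, prints its name and records it in a type-to-name map, both readable through getters and reset by SetClean.
; SetSelectedItemPrice pushes the stored item's price to the shop sub-widget's cost text.
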(event EventBeginPlay
  (bind _returnvalue (UserInterface|CreateWidget "/Game/MobileTest/Widget/W_TouchHud.W_TouchHud_C"))
  (bind _output_get (Variables|Default|SetWidgetHud _returnvalue))
  (UserInterface|Viewport|AddtoViewport _output_get 0))

(event Collision|EventActorBeginOverlap
  (params (OtherActor :type Actor%20Object%20Reference)))

(event EventTick
  (params (DeltaSeconds :type Float%20%28single-precision%29)))

(fn ConstructionScript)

(fn SetItemStruct
  (params (IconStruct :type ST%20Shop%20Own%20Struct%20Structure))
  ;[1 1 1] type 열거형으로 바꾸기
  (bind _output_get (Variables|Default|SetST_ItemStuct IconStruct))
  (Development|PrintString (.itemname _output_get))
  (Utilities|Map|Add (Variables|Default|Getstringmesh) (.itemtype _output_get) (.itemname _output_get)))

(fn GetItemStruct
  (return (Variables|Default|GetST_ItemStuct)))

(fn GetItemName
  (return (Variables|Default|Getstringmesh)))

(fn SetClean
  (Variables|Default|SetST_ItemStuct "")
  (Utilities|Map|Clear (Variables|Default|Getstringmesh)))

(fn SetSelectedItemPrice
  (Default|SetTextCost (Variables|/Game/MobileTest/Widget/W_TouchHud.W_TouchHud_C|GetW_Shop (Variables|Default|GetWidgetHud)) (Utilities|Text|ToText(Integer) (.itemprice (Variables|Default|GetST_ItemStuct)))))