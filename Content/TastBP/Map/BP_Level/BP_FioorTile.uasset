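; Floor tile for an endless-runner style minigame that populates itself and extends the track as the player passes over it.
; Construction scatters score-up child actors randomly inside ScoreUPArea, and BeginPlay spawns a random actor from the Class array at TrackPoints.
; When the touch character hits EndTrigger, it asks MiniGameMode to add a tile, then destroys itself after a delay.
; SetTrackPoints and SpawnBlocker are unwired in construction.
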(event OnComponentBeginOverlap(EndTrigger)
  (params (OverlappedComponent :type Primitive%20Component%20Object%20Reference) (OtherActor :type Actor%20Object%20Reference) (OtherComp :type Primitive%20Component%20Object%20Reference) (OtherBodyIndex :type Integer) (bFromSweep :type Boolean) (SweepResult :type Hit%20Result%20Structure%20%28by%20ref%29))
  (Utilities|Casting|CastToBP_Test_TouchCharacter OtherActor)
  (bind _asmini_game_mode (Utilities|Casting|CastToMiniGameMode (Game|GetGameMode)))
  (Default|AddFloorTile _asmini_game_mode)
  (Utilities|FlowControl|Delay 4.0)
  (Actor|DestroyActor))

(event EventBeginPlay
  (bind _class (Variables|Default|GetClass))
  (Game|SpawnActorfromClass (Utilities|Array|Get(acopy) _class (Math|Random|RandomIntegerinRange 0 (Utilities|Array|LastIndex _class))) (Variables|Default|GetTrackPoints) "Undefined" 0 0))

(event Collision|EventActorBeginOverlap
  (params (OtherActor :type Actor%20Object%20Reference)))

(event EventTick
  (params (DeltaSeconds :type Float%20%28single-precision%29)))

(fn ConstructionScript
  (CallFunction|SpawnScoreUp))

(fn GetAttachTransform
  (return (Transformation|GetWorldTransform (Variables|Default|GetAttackPoint))))

(fn SetTrackPoints
  (Variables|Default|SetTrackPoints (Transformation|GetRelativeTransform (Variables|Default|GetTrackPoint))))

(fn SpawnBlocker
  (AddComponent|AddChildActorComponent false (Variables|Default|GetTrackPoints)))

(fn SpawnScoreUp
  (bind _scoreuparea (Variables|Default|GetScoreUPArea))
  (for _index (range 0 5)
    (AddComponent|AddChildActorComponent false (Math|Conversions|ToTransform(Vector) (Math|Random|RandomPointinBoundingBox (Variables|/Script/Engine.SceneComponent|GetRelativeLocation _scoreuparea) (Variables|/Script/Engine.BoxComponent|GetBoxExtent _scoreuparea))))))