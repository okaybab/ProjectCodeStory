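; Portal actor that teleports an overlapping BP_TouchCharacter to the Spawn point of its linked portal.
; On BeginPlay it sets its text label and, by Lobby or Lecture type, assigns a scene capture render target and the opposite portal's material to its surface, so each portal displays the other's view.
; On overlap it disables the IsPotal flag on both portals for one second to prevent an immediate bounce back.
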(event OnComponentBeginOverlap(potalstatic)
  (params (OverlappedComponent :type Primitive%20Component%20Object%20Reference) (OtherActor :type Actor%20Object%20Reference) (OtherComp :type Primitive%20Component%20Object%20Reference) (OtherBodyIndex :type Integer) (bFromSweep :type Boolean) (SweepResult :type Hit%20Result%20Structure%20%28by%20ref%29))
  (bind _linkpotal (Variables|Default|GetLinkPotal))
  (bind _asbp_touch_character (Utilities|Casting|CastToBP_TouchCharacter OtherActor))
  (Utilities|IsValid _linkpotal
    (:Is%20Valid
      (if (Variables|Default|GetIsPotal)
        (CallFunction|SetPotalCollision false)
        (Transformation|SetActorLocation _asbp_touch_character (Transformation|GetWorldLocation (Variables|BP_Potal_C|Getspawn _linkpotal)) false true)
        (Utilities|FlowControl|Delay 1.0)
        (CallFunction|SetPotalCollision true)))))

(event OnComponentEndOverlap(potalstatic)
  (params (OverlappedComponent :type Primitive%20Component%20Object%20Reference) (OtherActor :type Actor%20Object%20Reference) (OtherComp :type Primitive%20Component%20Object%20Reference) (OtherBodyIndex :type Integer)))

(event Custom|SetPotalCollision
  (params (IsPotal :type Boolean))
  (Variables|Default|SetIsPotal IsPotal)
  (Variables|BP_Potal_C|SetIsPotal (Variables|Default|GetLinkPotal) IsPotal))

(event EventBeginPlay
  (bind _potalstatic (Variables|Default|Getpotalstatic))
  (bind _scenecapturecomponent2d (Variables|Default|GetSceneCaptureComponent2D))
  (Rendering|Components|TextRender|SetText (Variables|Default|GetTextRender) (Variables|Default|Gettext))
  (switch Utilities|FlowControl|Switch|SwitchonEnum_potal (Variables|Default|Getenum_linkpotal)
    (:NewEnumerator0
      (Variables|/Script/Engine.SceneCaptureComponent2D|SetTextureTarget _scenecapturecomponent2d "/Game/TastBP/BPPotal/RT_Potal1.RT_Potal1")
      (Rendering|Material|SetMaterial _potalstatic 0 "/Game/TastBP/BPPotal/RT_Potal2_Mat.RT_Potal2_Mat"))
    (:NewEnumerator1
      (Variables|/Script/Engine.SceneCaptureComponent2D|SetTextureTarget _scenecapturecomponent2d "/Game/TastBP/BPPotal/RT_Potal2.RT_Potal2")
      (Rendering|Material|SetMaterial _potalstatic 0 "/Game/TastBP/BPPotal/RT_Potal1_Mat.RT_Potal1_Mat"))))

(event Collision|EventActorBeginOverlap
  (params (OtherActor :type Actor%20Object%20Reference)))

(event EventTick
  (params (DeltaSeconds :type Float%20%28single-precision%29)))

(fn ConstructionScript)

(fn SetAcotorLocation)