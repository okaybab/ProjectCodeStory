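; BP_ScoreUP is a score pickup actor in the CookiRun game that awards coins to the player on touch.
; Its Sphere overlap casts to BP_Test_TouchCharacter and, if that character is not dead, calls AddCoin with CoinNum and destroys the pickup.
; A separate AddScore function raises UpScore by a fixed step and returns it, but nothing in this Blueprint calls it.
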(event OnComponentBeginOverlap(Sphere)
  (params (OverlappedComponent :type Primitive%20Component%20Object%20Reference) (OtherActor :type Actor%20Object%20Reference) (OtherComp :type Primitive%20Component%20Object%20Reference) (OtherBodyIndex :type Integer) (bFromSweep :type Boolean) (SweepResult :type Hit%20Result%20Structure%20%28by%20ref%29))
  (bind _asbp_test_touch_character (Utilities|Casting|CastToBP_Test_TouchCharacter OtherActor))
  (if (not (Variables|/Game/TastBP/CookiRun/GameMode/BP_Test_TouchCharacter.BP_Test_TouchCharacter_C|GetIsDeath _asbp_test_touch_character))
    (Default|AddCoin _asbp_test_touch_character (Variables|Default|GetCoin%20Num))
    (Actor|DestroyActor)))

(event EventBeginPlay)

(event Collision|EventActorBeginOverlap
  (params (OtherActor :type Actor%20Object%20Reference)))

(event EventTick
  (params (DeltaSeconds :type Float%20%28single-precision%29)))

(fn ConstructionScript)

(fn AddScore
  (bind _output_get (Variables|Default|SetUpScore (+ (Variables|Default|GetUpScore) 1e+01)))
  (return _output_get))