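; BP_Keeper is an actor whose static mesh swings in yaw in response to the player's P key.
; On BeginPlay it binds to Mini_Pawn's P pressed and released dispatchers, each starting a looping 0.01-second timer.
; The press timer adds Speed-scaled yaw until it exceeds 90 degrees.
; The release timer decrements Speed each tick and applies it as yaw until yaw drops below zero.
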(event Custom|TimerTargetAttack
  (Utilities|Time|SetTimerbyFunctionName 0 "PressedPkey" 0.01 true))

(event Custom|ReleasedP
  (Utilities|Time|SetTimerbyFunctionName 0 "ReleasedPKey" 0.01 true))

(event EventBeginPlay
  (bind _asmini_pawn (Utilities|Casting|CastToMini_Pawn (Game|Player|GetPlayerPawn 0)))
  (EventDispatchers|BindEventtoEventDispatcherPKeyPressed _asmini_pawn (delegate Custom|TimerTargetAttack))
  (EventDispatchers|BindEventtoEventDispatcherPKeyReleased _asmini_pawn (delegate Custom|ReleasedP)))

(fn ConstructionScript)

(fn PressedPkey
  (Transformation|AddWorldRotation (Variables|Default|GetStaticMesh) (Math|Rotator|MakeRotator 0.0 0.0 (* 0.01 (Variables|Default|GetSpeed))) false false)
  (if (not (<= (.yaw (Transformation|GetWorldRotation (Variables|Default|GetStaticMesh))) 9e+01))
    (Utilities|Time|ClearTimerbyFunctionName 0 "PressedPkey")
    (Development|PrintString "Hello")))

(fn ReleasedPKey
  (bind _result (Math|Float|DecrementFloat (Variables|Default|GetSpeed))
    (:%20%20
      (Transformation|AddWorldRotation (Variables|Default|GetStaticMesh) (Math|Rotator|MakeRotator 0.0 0.0 (* _result 0.01)) false false)
      (if (not (<= 0.0 (.yaw (Transformation|GetWorldRotation (Variables|Default|GetStaticMesh)))))
        (Utilities|Time|ClearTimerbyFunctionName 0 "ReleasedPKey")))))