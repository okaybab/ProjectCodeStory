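; BP_Mini_Track0 is a jump-track piece for the CookiRun game that damages the player on contact.
; A mesh overlap with a living BP_Test_TouchCharacter applies Damage0 and destroys the actor; hit effect and sound nodes are disconnected.
; TrackPoint exposes the Arrow's world transform.
; HPUpdate passes Damage0 to UpdateHP in hundredths until the total is reached, then clears its timer, though nothing here starts that timer.
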(event OnComponentBeginOverlap(StaticMesh)
  (params (OverlappedComponent :type Primitive%20Component%20Object%20Reference) (OtherActor :type Actor%20Object%20Reference) (OtherComp :type Primitive%20Component%20Object%20Reference) (OtherBodyIndex :type Integer) (bFromSweep :type Boolean) (SweepResult :type Hit%20Result%20Structure%20%28by%20ref%29))
  (bind _asbp_test_touch_character (Utilities|Casting|CastToBP_Test_TouchCharacter OtherActor))
  (if (not (Variables|/Game/TastBP/CookiRun/GameMode/BP_Test_TouchCharacter.BP_Test_TouchCharacter_C|GetIsDeath _asbp_test_touch_character))
    (Game|Damage|ApplyDamage _asbp_test_touch_character (Variables|Default|GetDamage_0) 0 0)
    (Actor|DestroyActor)))

(event EventBeginPlay)

(event Collision|EventActorBeginOverlap
  (params (OtherActor :type Actor%20Object%20Reference)))

(fn ConstructionScript)

(fn TrackPoint
  (return (Transformation|GetWorldTransform (Variables|Default|GetArrow))))

(fn HPUpdate
  (bind _damage_0 (Variables|Default|GetDamage_0))
  (bind _returnvalue (/ _damage_0 1e+02))
  (LocalVariables|SetUpdateHP _returnvalue)
  (bind _output_get (Variables|Default|SetTotalDamage (+ _returnvalue (Variables|Default|GetTotalDamage))))
  (if (<= _output_get (Variables|Default|GetDamage_0))
    (CallFunction|UpdateHP (LocalVariables|GetUpdateHP))
    (Development|PrintString (Utilities|String|ToString(Float) (Variables|Default|GetTotalDamage)) true true "(R=0.963901,G=1.000000,B=0.000000,A=1.000000)")
    (else
      (Utilities|Time|ClearTimerbyFunctionName 0 "HPUpdate"))))